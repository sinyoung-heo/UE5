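; BP_Knight is a 2D knight Blueprint that turns its sprite to face the direction of player input.
; MoveUp and MoveRight axis events check the input sign and swap the Sprite's flipbook between up, down and side idle animations.
; One side flipbook serves both horizontal directions by rotating the Sprite 180 degrees for left.
; The graph applies no movement, and BeginPlay, Tick and overlap events are empty.
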(event `InputAxis|MoveUp`
  (params (AxisValue :type "Float (single-precision)"))
  (bind _sprite (`self.Sprite`))
  (`/Engine/EditorBlueprintResources/StandardMacros.CompareFloat` AxisValue
    (:`>`
      (`PaperFlipbookComponent.SetFlipbook` _sprite "/Game/Sprites/Knight/up_idle.up_idle"))
    (:`<`
      (`PaperFlipbookComponent.SetFlipbook` _sprite "/Game/Sprites/Knight/down_idle.down_idle"))))

(event `InputAxis|MoveRight`
  (params (AxisValue :type "Float (single-precision)"))
  (bind _sprite (`self.Sprite`))
  (`/Engine/EditorBlueprintResources/StandardMacros.CompareFloat` AxisValue
    (:`>`
      (`PaperFlipbookComponent.SetFlipbook` _sprite "/Game/Sprites/Knight/side_idle.side_idle")
      (`SceneComponent.K2_SetRelativeRotation` _sprite (struct) false false))
    (:`<`
      (`PaperFlipbookComponent.SetFlipbook` _sprite "/Game/Sprites/Knight/side_idle.side_idle")
      (`SceneComponent.K2_SetRelativeRotation` _sprite (struct :`Yaw` 180.0) false false))))

(fn `UserConstructionScript`)