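; BP_Slime is a slime actor that travels along world +X at a randomly chosen speed.
; On BeginPlay, InitSpeed rolls the speed within a fixed range and prints it with the slime's name.
; Tick calls Move, which offsets the location by speed and delta time without sweeping.
; An actor overlap sets the Arrived flag, but movement does not check it, so the slime keeps moving.
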(event `self.ReceiveBeginPlay`
  (`self.InitSpeed`))

(event `self.ReceiveActorBeginOverlap`
  (params (OtherActor :type "Actor Object Reference"))
  (set `self.bArrived` true))

(event `self.ReceiveTick`
  (params (DeltaSeconds :type "Float (single-precision)"))
  (`self.Move` DeltaSeconds))

(fn `InitSpeed`
  (set `self.Speed` (`KismetMathLibrary.RandomFloatInRange` 300.0 3000.0))
  (`KismetSystemLibrary.PrintText` (`|FormatText` "{name} : speed {speed}" (`self.Name`) (`KismetMathLibrary.Conv_DoubleToInt64` (`self.Speed`)))))

(fn `Move`
  (params (DeltaSeconds :type "Float (double-precision)"))
  (`self.K2_SetActorLocation` (+ (`self.K2_GetActorLocation`) (* (* DeltaSeconds (`self.Speed`)) (`KismetMathLibrary.MakeVector` 1.0)))))

(fn `UserConstructionScript`)